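; BPC_Dégâts is a damage component that tracks hit points and signals death for the actor that owns it.
; PrendreDégâts subtracts the incoming amount from PV, clamped between zero and PVMax, and ignores hits once Meurt is set.
; When PV reaches zero, it sets Meurt, fires the ALaMort dispatcher and returns true to the caller.
; BeginPlay and Tick are unused.
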(fn `Prendre Dégâts`
  (params (`Quantité` :type "Float (double-precision)"))
  (returns (`Dégâts subis` :type Boolean))
  (if (not (`self.Meurt`))
    (bind _output_get (set `self.PV ` (`KismetMathLibrary.FClamp` (- (`self.PV `) `Quantité`) 0.0 (`self.PV max`))))
    (if (== _output_get 0.0)
      (set `self.Meurt` true)
      (`self.A la mort`)
      (return true))))